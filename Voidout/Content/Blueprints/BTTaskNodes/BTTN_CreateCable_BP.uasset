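; Behavior tree task for the shadow explorer that cables a path point's torch or tower to its neighbors and flags the point as having a lamp post.
; It takes the index from the blackboard and the path from the pawn, skipping beams for points inside light.
; Previous and next points get laser-cable particle beams if they are path endpoints or already flagged.
; Beams to non-endpoints re-attach to the neighbor's energy torch, and the task always reports success.
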(event EventReceiveExecute
  (params (OwnerActor :type Actor%20Object%20Reference))
  (bind _paramsok (CallFunction|CheckInitialParams OwnerActor))
  (if _paramsok
    (if (Variables|/Script/Voidout.TGPT_Explorer|Getm_isInsideLight (Utilities|Array|Get(acopy) (Variables|Default|Getpath_copy) (Variables|Default|Getindex)))
      _
      (else
        (CallFunction|CreateCable 1)
        (CallFunction|CreateCable -1)))
    (Variables|/Script/Voidout.TGPT_Explorer|Setm_haveLampPost (Utilities|Array|Get(acopy) (Variables|Default|Getpath_copy) (Variables|Default|Getindex)) true)
    (AI|BehaviorTree|FinishExecute true)
    (else
      (AI|BehaviorTree|FinishExecute true))))

(fn CreateCable
  (params (indextTo_compare :type Integer))
  (bind _output_get (Variables|Default|Setnext%20index (+ (Variables|Default|Getindex) indextTo_compare)))
  (bind _isinsidevector (CallFunction|CheckIndexinVector _output_get))
  (if _isinsidevector
    (bind _isbound (CallFunction|CheckBoundariesArray _output_get))
    (if _isbound
      _
      (elif (Variables|/Script/Voidout.TGPT_Explorer|Getm_haveLampPost (Utilities|Array|Get(acopy) (Variables|Default|Getpath_copy) (Variables|Default|Getnext%20index)))
        _
        (else
          (return))))
    (bind _isok (CallFunction|SetBeamLocationVariables _isbound (Variables|Default|Getindex) (Variables|Default|Getnext%20index)))
    (if _isok
      (CallFunction|CreateBeam)
      (return)
      (else
        (return)))
    (else
      (return))))

(fn CheckBoundariesArray
  (params (index_to_check :type Integer))
  (if (or (< index_to_check 0) (>= index_to_check (Utilities|Array|Length (Variables|Default|Getpath_copy))))
    (return false)
    (else
      (return (or (== index_to_check 0) (== index_to_check (- (Utilities|Array|Length (Variables|Default|Getpath_copy)) 1)))))))

(fn CheckIndexinVector
  (params (indexToCompare :type Integer))
  (return (and (>= indexToCompare 0) (< indexToCompare (Utilities|Array|Length (Variables|Default|Getpath_copy))))))

(fn SetBeamLocationVariables
  (params (isBound :type Boolean) (actualIndex :type Integer) (nextIndex :type Integer))
  (bind _path_copy (Variables|Default|Getpath_copy))
  (bind _output (Utilities|Array|Get(acopy) _path_copy nextIndex))
  (bind _returnvalue (Transformation|GetActorLocation _output))
  (bind (_x _y _z) (Math|Vector|BreakVector _returnvalue))
  (bind _isok (CallFunction|MakeLocationVector actualIndex true))
  (if _isok
    (if isBound
      (Variables|Default|Settarget (Math|Vector|MakeVector _x _y (+ _z 1e+01)))
      (else
        (bind _isok_2 (CallFunction|MakeLocationVector nextIndex false))
        (if _isok_2
          (bind _asactr_energy_torche_bp (Utilities|Casting|CastToACTR_EnergyTorche_BP (Class|TGPTExplorer|GetTorcheorTower _output)))
          (Variables|Default|Setparent_for_beam _asactr_energy_torche_bp)
          (else
            (return false)))))
    (return true)
    (else
      (return false))))

(fn CheckInitialParams
  (params (owner :type Object%20Object%20Reference))
  (bind _targetpointposition (Variables|Default|GetTargetPointPosition))
  (bind _returnvalue (Class|BTFunctionLibrary|GetBlackboardValueasInt _targetpointposition))
  (bind _asaict_explorer_bp (Utilities|Casting|CastToAICT_Explorer_BP owner)
    (:then
      (bind _aschrt_shadow_explorer_bp (Utilities|Casting|CastToCHRT_ShadowExplorer_BP (Pawn|GetControlledPawn _asaict_explorer_bp))
        (:then
          (Variables|Default|Setpath_copy (Variables|/Script/Voidout.CHRT_Explorer|Getm_path _aschrt_shadow_explorer_bp))
          (bind _isinsidevector (CallFunction|CheckIndexinVector _returnvalue))
          (if _isinsidevector
            (Variables|Default|Setindex _returnvalue)
            (return (not (Variables|/Script/Voidout.TGPT_Explorer|Getm_haveLampPost (Utilities|Array|Get(acopy) (Variables|Default|Getpath_copy) (Variables|Default|Getindex)))))
            (else
              (return false))))
        (:CastFailed
          _)))
    (:CastFailed
      _))
  (return false))

(fn CreateBeam
  (bind _returnvalue (Effects|SpawnEmitterAttached "/Game/ParticleSystems/PSYS_LaserCable.PSYS_LaserCable" (Variables|/Script/Engine.Actor|GetRootComponent (Class|TGPTExplorer|GetTorcheorTower (Utilities|Array|Get(acopy) (Variables|Default|Getpath_copy) (Variables|Default|Getindex)))) "None" (Variables|Default|Getsource) "0, 0, 0" "1.000000,1.000000,1.000000" "KeepRelativeOffset" false))
  (Class|ParticleSystemComponent|SetBeamSourcePoint _returnvalue 0 (Variables|Default|Getsource))
  (Class|ParticleSystemComponent|SetBeamTargetPoint _returnvalue 0 (Variables|Default|Gettarget))
  (if (Utilities|IsValid (Variables|Default|Getparent_for_beam))
    (Transformation|AttachComponentToComponent _returnvalue (Variables|/Script/Engine.Actor|GetRootComponent (Variables|Default|Getparent_for_beam)) "None" "KeepRelative" "KeepRelative" "KeepRelative" true)
    (Variables|Default|Setparent_for_beam 0)
    (return)))

(fn MakeLocationVector
  (params (index :type Integer) (isSource :type Boolean))
  (bind _path_copy (Variables|Default|Getpath_copy))
  (bind _output (Utilities|Array|Get(acopy) _path_copy index))
  (bind _returnvalue (Class|TGPTExplorer|GetTorcheorTower _output))
  (bind _returnvalue_2 (Transformation|GetActorLocation _output))
  (bind _returnvalue_3 (Transformation|GetActorLocation _returnvalue))
  (bind _z (Math|Vector|BreakVector _returnvalue_2))
  (bind (_x _y) (Math|Vector|BreakVector _returnvalue_3))
  (bind _returnvalue_4 (+ _z 1e+01))
  (bind _returnvalue_5 (Math|Vector|MakeVector _x _y _returnvalue_4))
  (if (Utilities|IsValid _returnvalue)
    (if isSource
      (Variables|Default|Setsource _returnvalue_5)
      (else
        (Variables|Default|Settarget _returnvalue_5)))
    (return true)
    (else
      (return false))))