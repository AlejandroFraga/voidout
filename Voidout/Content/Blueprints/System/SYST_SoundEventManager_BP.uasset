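; Central FMOD sound manager exposing named play and stop calls for player, enemy, structure, ambient and menu audio.
; Most calls fire 2D or positioned one-shot events, while several step, ambient, creation and damage hooks are empty.
; LoopSound tracks instances by position so tower damage loops can be stopped.
; Music functions control buses and remember the last track to resume after sequence music; SetMasterVolume actually sets the Music bus.
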(event EventBeginPlay)

(event EventStopFightMusic
  (CallFunction|PlayMusic false))

(event EventPlayGeneralAmbient
  (Class|FMODBlueprintStatics|PlayEvent2D "/Game/FMOD/Events/Sound_Effects/AmbientSound2D.AmbientSound2D"))

(event EventPlayMusicBus
  (Class|FMODBlueprintStatics|BusSetPaused "/Game/FMOD/Buses/Master/Music.Music" false))

(event EventPauseMusicBus
  (Class|FMODBlueprintStatics|BusSetPaused "/Game/FMOD/Buses/Master/Music.Music" true))

(event EventPlayAmbient01
  (params (position :type Vector :default "0, 0, 0"))
  (Class|FMODBlueprintStatics|PlayEvent2D "/Game/FMOD/Events/Sound_Effects/AmbientSound2D.AmbientSound2D"))

(event EventPlayFight01
  (params (position :type Vector :default "0, 0, 0"))
  (Class|FMODBlueprintStatics|PlayEventatLocation 0 (Math|Conversions|ToTransform(Vector) position)))

(event EventPlayUnreadySkill
  (Class|FMODBlueprintStatics|PlayEvent2D "/Game/FMOD/Events/Sound_Effects/UnreadySkill2D.UnreadySkill2D"))

(event EventPlayCommanderDamage
  (params (position :type Vector :default "0, 0, 0"))
  (Class|FMODBlueprintStatics|PlayEventatLocation "/Game/FMOD/Events/Sound_Effects/CommanderAttack3D.CommanderAttack3D" (Math|Conversions|ToTransform(Vector) position)))

(event EventPlayCommanderDeath
  (params (position :type Vector :default "0, 0, 0"))
  (Class|FMODBlueprintStatics|PlayEventatLocation "/Game/FMOD/Events/Sound_Effects/CommanderDeath_3D.CommanderDeath_3D" (Math|Conversions|ToTransform(Vector) position)))

(event EventPlayCommanderSteps
  (params (position :type Vector :default "0, 0, 0")))

(event EventPlayEnergyBarrierAmbient
  (params (position :type Vector :default "0, 0, 0")))

(event EventPlayEnergyBarrierDamage
  (params (position :type Vector :default "0, 0, 0"))
  (Class|FMODBlueprintStatics|PlayEventatLocation "/Game/FMOD/Events/Sound_Effects/EnergyBarrier3D.EnergyBarrier3D" (Math|Conversions|ToTransform(Vector) position)))

(event EventPlayEnergyBarrierOff
  (params (position :type Vector :default "0, 0, 0"))
  (Class|FMODBlueprintStatics|PlayEventatLocation "/Game/FMOD/Events/Sound_Effects/EnergyBarrierOff3D.EnergyBarrierOff3D" (Math|Conversions|ToTransform(Vector) position)))

(event EventPlayEnergyBarrieron
  (params (position :type Vector :default "0, 0, 0")))

(event EventPlayLightTrooperDeath
  (params (position :type Vector :default "0, 0, 0"))
  (Class|FMODBlueprintStatics|PlayEventatLocation "/Game/FMOD/Events/Sound_Effects/MyLightTrooperDeath_3D.MyLightTrooperDeath_3D" (Math|Conversions|ToTransform(Vector) position)))

(event EventPlayLightTrooperShoot
  (params (position :type Vector :default "0, 0, 0"))
  (Class|FMODBlueprintStatics|PlayEventatLocation "/Game/FMOD/Events/Sound_Effects/LightTrooperShoot3D.LightTrooperShoot3D" (Math|Conversions|ToTransform(Vector) position)))

(event EventPlayLightTrooperSteps
  (params (position :type Vector :default "0, 0, 0")))

(event EventPlayShadowExplorerDeath
  (params (position :type Vector :default "0, 0, 0"))
  (Class|FMODBlueprintStatics|PlayEventatLocation "/Game/FMOD/Events/Sound_Effects/ExplorerDeath3D.ExplorerDeath3D" (Math|Conversions|ToTransform(Vector) position)))

(event EventPlayShadowExplorerShoot
  (params (position :type Vector :default "0, 0, 0"))
  (Class|FMODBlueprintStatics|PlayEventatLocation "/Game/FMOD/Events/Sound_Effects/Shot01_3D.Shot01_3D" (Math|Conversions|ToTransform(Vector) position)))

(event EventPlayShadowExplorerSteps
  (params (position :type Vector :default "0, 0, 0")))

(event EventPlayEnergyCoreAmbient
  (params (position :type Vector :default "0, 0, 0")))

(event EventPlayEnergyCoreCreated
  (params (position :type Vector :default "0, 0, 0")))

(event EventPlayEnergyCoreDamage
  (params (position :type Vector :default "0, 0, 0")))

(event EventPlayEnergyCoreDestruction
  (params (position :type Vector :default "0, 0, 0"))
  (Class|FMODBlueprintStatics|PlayEventatLocation "/Game/FMOD/Events/Sound_Effects/GeneratorDestruction3D.GeneratorDestruction3D" (Math|Conversions|ToTransform(Vector) position)))

(event EventPlayEnergyTorchAmbient
  (params (position :type Vector :default "0, 0, 0")))

(event EventPlayEnergyTorchCreated
  (params (position :type Vector :default "0, 0, 0")))

(event EventPlayEnergyTorchDamage
  (params (position :type Vector :default "0, 0, 0")))

(event EventPlayEnergyTorchDestruction
  (params (position :type Vector :default "0, 0, 0"))
  (Class|FMODBlueprintStatics|PlayEventatLocation "/Game/FMOD/Events/Sound_Effects/TorchDestruction_3D.TorchDestruction_3D" (Math|Conversions|ToTransform(Vector) position)))

(event EventPlayPlayerDeath
  (params (position :type Vector :default "0, 0, 0"))
  (Class|FMODBlueprintStatics|PlayEvent2D "/Game/FMOD/Events/Sound_Effects/PlayerDeath2D.PlayerDeath2D"))

(event EventPlayAbilitySDCharged
  (Class|FMODBlueprintStatics|PlayEvent2D "/Game/FMOD/Events/Sound_Effects/ShadowDashReload2D.ShadowDashReload2D"))

(event EventPlayPlayerDamage
  (params (position :type Vector :default "0, 0, 0"))
  (Class|FMODBlueprintStatics|PlayEvent2D "/Game/FMOD/Events/Sound_Effects/CharacterHurt2D.CharacterHurt2D"))

(event EventPlayPlayerDarkSlash
  (params (position :type Vector :default "0, 0, 0"))
  (Class|FMODBlueprintStatics|PlayEventatLocation "/Game/FMOD/Events/Sound_Effects/PlayerAttack3D.PlayerAttack3D" (Math|Conversions|ToTransform(Vector) position)))

(event EventPlayPlayerShadowDash
  (params (position :type Vector :default "0, 0, 0"))
  (Class|FMODBlueprintStatics|PlayEventatLocation "/Game/FMOD/Events/Sound_Effects/ShadowDash02_3D.ShadowDash02_3D" (Math|Conversions|ToTransform(Vector) position)))

(event EventPlayPlayerSteps
  (params (position :type Vector :default "0, 0, 0"))
  (Class|FMODBlueprintStatics|PlayEvent2D "/Game/FMOD/Events/Sound_Effects/CharacterMovement2D.CharacterMovement2D"))

(event EventPlayPlayerVoidout
  (params (position :type Vector :default "0, 0, 0"))
  (Class|FMODBlueprintStatics|PlayEventatLocation "/Game/FMOD/Events/Sound_Effects/VoidOut3D.VoidOut3D" (Math|Conversions|ToTransform(Vector) position)))

(event EventPlayEnergyTowerDestruction
  (params (position :type Vector :default "0, 0, 0")))

(event EventPlayEnergyTowerAmbient
  (params (position :type Vector :default "0, 0, 0")))

(event EventPlayEnergyTowerCreation
  (params (position :type Vector :default "0, 0, 0")))

(event EventPlayEnergyTowerDamage
  (params (position :type Vector :default "0, 0, 0"))
  (CallFunction|LoopSound "/Game/FMOD/Events/Sound_Effects/TowerDamage3D.TowerDamage3D" position true))

(event EventStopEnergyTowerDamage
  (params (position :type Vector :default "0, 0, 0"))
  (CallFunction|LoopSound "/Game/FMOD/Events/Sound_Effects/TowerDamage3D.TowerDamage3D" position false))

(event EventPlayPowerGeneratorAmbient
  (params (position :type Vector :default "0, 0, 0")))

(event EventPlayPowerGeneratorCreated
  (params (position :type Vector :default "0, 0, 0")))

(event EventPlayPowerGeneratorDamage
  (params (position :type Vector :default "0, 0, 0")))

(event EventPlayPowerGeneratorDestruction
  (params (position :type Vector :default "0, 0, 0"))
  (Class|FMODBlueprintStatics|PlayEventatLocation "/Game/FMOD/Events/Sound_Effects/GeneratorDestruction3D.GeneratorDestruction3D" (Math|Conversions|ToTransform(Vector) position)))

(fn ConstructionScript)

(fn LoopSound
  (params (SoundEvent :type FMOD%20Event%20Object%20Reference) (Position :type Vector%20%28by%20ref%29) (isPlay? :type Boolean))
  (if isPlay?
    (bind _returnvalue (Class|FMODBlueprintStatics|PlayEventatLocation SoundEvent (Math|Conversions|ToTransform(Vector) Position) false))
    (bind _returnvalue_2 (Utilities|Array|Add (Variables|Default|Getsounds) _returnvalue))
    (Utilities|Map|Add (Variables|Default|GetIndexPositions) _returnvalue_2 Position)
    (Class|FMODBlueprintStatics|EventInstancePlay _returnvalue)
    (else
      (for (_array_element _array_index) (Variables|Default|Getsounds)
        (if (Math|Vector|Equal(Vector) (.Value (Utilities|Map|Find (Variables|Default|GetIndexPositions) _array_index)) Position 0.0001)
          (Class|FMODBlueprintStatics|EventInstanceStop _array_element true)
          (Utilities|Map|Remove (Variables|Default|GetIndexPositions) _array_index))))))

(fn GetPlayerAnimInstance
  (bind _returnvalue (Game|GetPlayerCharacter 0))
  (bind _mesh (Variables|/Script/Engine.Character|GetMesh _returnvalue))
  (bind _returnvalue_2 (Components|SkeletalMesh|GetAnimInstance _mesh))
  ;[1 1 1] We get the Character and check if it's valid
  (if (Utilities|IsValid _returnvalue)
    ;[1 1 1] We get the Character Mesh and check if it's valid
    (if (Utilities|IsValid _mesh)
      ;[1 1 1] We get the Character Mesh Anim Instance and check if it's valid
      (if (Utilities|IsValid _returnvalue_2)
        ;[1 1 1] Cast
        (bind _asanim_player_bp (Utilities|Casting|CastToANIM_Player_BP _returnvalue_2)
          (:CastFailed
            (return _asanim_player_bp)))
        (else
          _))))
  (return 0))

(fn PlayMenuSelection
  (Class|FMODBlueprintStatics|PlayEvent2D "/Game/FMOD/Events/Sound_Effects/MenuSelect2D.MenuSelect2D"))

(fn PlayMenuBack
  (Class|FMODBlueprintStatics|PlayEvent2D "/Game/FMOD/Events/Sound_Effects/MenuSelect2D.MenuSelect2D"))

(fn PlayMenuMovement
  (Class|FMODBlueprintStatics|PlayEvent2D "/Game/FMOD/Events/Sound_Effects/MenuMovement2D.MenuMovement2D"))

(fn PlayMenuStartButton
  (Class|FMODBlueprintStatics|PlayEvent2D "/Game/FMOD/Events/Sound_Effects/MenuStart2D.MenuStart2D"))

(fn PlayMusic
  (params (isPlay? :type Boolean) (Event :type FMOD%20Event%20Object%20Reference))
  (if isPlay?
    (Variables|Default|SetlastEventPlayed Event)
    (Class|FMODBlueprintStatics|BusSetPaused "/Game/FMOD/Buses/Master/Music.Music" false)
    (Class|FMODBlueprintStatics|BusStopAllEvents "/Game/FMOD/Buses/Master/Music.Music" "ALLOWFADEOUT")
    (Class|FMODBlueprintStatics|PlayEvent2D Event)
    (else
      (Class|FMODBlueprintStatics|BusStopAllEvents "/Game/FMOD/Buses/Master/Music.Music" "ALLOWFADEOUT")
      (Class|FMODBlueprintStatics|PlayEvent2D "/Game/FMOD/Events/Sound_Effects/AmbientSound2D.AmbientSound2D")
      (Variables|Default|SetlastEventPlayed "/Game/FMOD/Events/Sound_Effects/AmbientSound2D.AmbientSound2D"))))

(fn PlayTowerCreation
  (params (Position :type Vector))
  (Class|FMODBlueprintStatics|PlayEventatLocation "/Game/FMOD/Events/Sound_Effects/TowerFall3D.TowerFall3D" (Math|Conversions|ToTransform(Vector) Position)))

(fn MasterVolume
  (params (Volume :type Float%20%28single-precision%29))
  (Class|FMODBlueprintStatics|BusSetVolume "/Game/FMOD/Buses/Master.Master" Volume))

(fn SetMasterVolume
  (params (volume :type Float%20%28single-precision%29))
  (Class|FMODBlueprintStatics|BusSetVolume "/Game/FMOD/Buses/Master/Music.Music" volume))

(fn SetMusicVolume
  (params (volume :type Float%20%28single-precision%29))
  (Class|FMODBlueprintStatics|BusSetVolume "/Game/FMOD/Buses/Master/Music.Music" volume))

(fn SetSoundsVolume
  (params (volume :type Float%20%28single-precision%29))
  (Class|FMODBlueprintStatics|BusSetVolume "/Game/FMOD/Buses/Master/Sound.Sound" volume))

(fn PlayCommanderAttack
  (params (Position :type Vector))
  (Class|FMODBlueprintStatics|PlayEventatLocation "/Game/FMOD/Events/Sound_Effects/CommanderAttack3D.CommanderAttack3D" (Math|Conversions|ToTransform(Vector) Position)))

(fn PlaySequenceMusic
  (params (Music :type FMOD%20Event%20Object%20Reference) (isForPlay? :type Boolean))
  (bind _lasteventplayed (Variables|Default|GetlastEventPlayed))
  (bind _sequencemusic (Variables|Default|GetSequenceMusic))
  (if isForPlay?
    (Class|FMODBlueprintStatics|BusSetPaused "/Game/FMOD/Buses/Master/Music.Music" false)
    ;[1 1 1] Cause sometimes FMOD start twice instead of one
    (bind _returnvalue (Class|FMODBlueprintStatics|PlayEvent2D Music))
    (Utilities|Array|Insert _sequencemusic _returnvalue (Utilities|Array|Length _sequencemusic))
    (else
      (for _array_element (Variables|Default|GetSequenceMusic)
        (Class|FMODBlueprintStatics|EventInstanceStop _array_element true))
      (if (Utilities|IsValid _lasteventplayed)
        (Class|FMODBlueprintStatics|PlayEvent2D _lasteventplayed)))))

(fn StopMusic
  (Class|FMODBlueprintStatics|BusStopAllEvents "/Game/FMOD/Buses/Master/Music.Music" "ALLOWFADEOUT"))