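; Falling tower actor that drops when the player first enters its trigger volume, with its spotlight switched off shortly after BeginPlay.
; The trigger enables mesh physics, applies a strong downward force and plays a tower sound through the sound event manager.
; The first hit freezes the mesh as query-only collision and plays controller rumble if the game instance allows vibration.
; Construction widens the spotlight's outer cone and flags it as a falling tower.
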(event OnComponentBeginOverlap(TriggerFall)
  (params (OverlappedComponent :type Primitive%20Component%20Object%20Reference) (OtherActor :type Actor%20Object%20Reference) (OtherComp :type Primitive%20Component%20Object%20Reference) (OtherBodyIndex :type Integer) (bFromSweep :type Boolean) (SweepResult :type Hit%20Result%20Structure%20%28by%20ref%29))
  (bind _staticmesh (Variables|Default|GetStaticMesh))
  ;[1 1 1] TriggerFall
  (if (not (Variables|Default|GetwasTriggered))
    (if (== OtherActor (Game|GetPlayerCharacter 0))
      (Variables|Default|SetwasTriggered true)
      (Physics|SetSimulatePhysics _staticmesh true)
      (Collision|SetCollisionEnabled _staticmesh "QueryAndPhysics")
      (Components|Activation|Deactivate (Variables|Default|GetTriggerFall))
      (Physics|AddForce (Variables|Default|GetStaticMesh) "0.000000, 0,-40000000.000000" "None" false)
      (bind _returnvalue (Actor|GetActorOfClass "/Game/Blueprints/System/SYST_SoundEventManager_BP.SYST_SoundEventManager_BP_C"))
      (Default|PlayTowerCreation _returnvalue (Transformation|GetActorLocation)))))

(event EventBeginPlay
  ;[1 1 1] Temporary Begin Play override to make if off permanent
  (Utilities|FlowControl|Delay 0.2)
  (Class|ACTRSwitchableLight|LightOffPermanent))

(event Collision|EventHit
  (params (MyComp :type Primitive%20Component%20Object%20Reference) (Other :type Actor%20Object%20Reference) (OtherComp :type Primitive%20Component%20Object%20Reference) (bSelfMoved :type Boolean) (HitLocation :type Vector :default "0, 0, 0") (HitNormal :type Vector :default "0, 0, 0") (NormalImpulse :type Vector :default "0, 0, 0") (Hit :type Hit%20Result%20Structure%20%28by%20ref%29))
  (bind _staticmesh (Variables|Default|GetStaticMesh))
  ;[1 1 1] Hit
  (if (not (Variables|Default|GethasFallen))
    (Variables|Default|SethasFallen true)
    (Physics|SetSimulatePhysics _staticmesh false)
    (Collision|SetCollisionEnabled _staticmesh "QueryOnly")
    (CallFunction|ForceFeedbackFalling)))

(fn ConstructionScript
  (bind _spotlight (Variables|Default|GetSpotLight))
  ;[1 1 1] Soluciona problemas de posicionamiento de las esferas de daño y para el movimiento de la IA.
  (Rendering|Lighting|SetOuterConeAngle _spotlight (+ (Variables|/Script/Engine.SpotLightComponent|GetInnerConeAngle _spotlight) 3.0))
  (Variables|Default|Setm_isFallingTower true))

(fn GetGMINBase
  (bind _asgmin_base (Utilities|Casting|CastToGMIN_Base (Game|GetGameInstance))
    (:then
      (return _asgmin_base))
    (:CastFailed
      (return _asgmin_base))))

(fn ForceFeedbackFalling
  (bind _gminbase (CallFunction|GetGMINBase))
  (if (and (Variables|/Script/Voidout.GMIN_Base|GetisUsingController _gminbase) (Variables|/Script/Voidout.GMIN_Base|GetisVibrationEnabled _gminbase))
    (Game|Feedback|ClientPlayForceFeedback (Game|GetPlayerController 0) "/Game/ForceFeedback/FFEF_EnergyTowerFalling.FFEF_EnergyTowerFalling" "Activated" false true true)
    (return)))