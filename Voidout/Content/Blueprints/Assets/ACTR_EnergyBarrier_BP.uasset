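; Energy barrier actor that handles collision end-overlaps and can play controller rumble for barrier hits.
; The collision component's end-overlap event, marked temporary, forwards to an EndOverlap function whose body is not defined here.
; ForceFeedbackHit checks controller use and vibration settings on the GMIN_Base game instance, then plays the hit effect on player 0, ignoring time dilation and pause.
; Nothing in this file calls ForceFeedbackHit.
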(event OnComponentEndOverlap(m_collisionComponent)
  (params (OverlappedComponent :type Primitive%20Component%20Object%20Reference) (OtherActor :type Actor%20Object%20Reference) (OtherComp :type Primitive%20Component%20Object%20Reference) (OtherBodyIndex :type Integer))
  ;[1 1 1] TEMPORARY: End Overlap
  (Class|ACTREnergyBarrier|EndOverlap OverlappedComponent OtherActor OtherComp OtherBodyIndex))

(fn ConstructionScript)

(fn GetGMINBase
  (bind _asgmin_base (Utilities|Casting|CastToGMIN_Base (Game|GetGameInstance))
    (:then
      (return _asgmin_base))
    (:CastFailed
      (return _asgmin_base))))

(fn ForceFeedbackHit
  (bind _gminbase (CallFunction|GetGMINBase))
  (if (and (Variables|/Script/Voidout.GMIN_Base|GetisUsingController _gminbase) (Variables|/Script/Voidout.GMIN_Base|GetisVibrationEnabled _gminbase))
    (Game|Feedback|ClientPlayForceFeedback (Game|GetPlayerController 0) "/Game/ForceFeedback/FFEF_EnergyBarrierHit.FFEF_EnergyBarrierHit" "Activated" false true true)
    (return)))