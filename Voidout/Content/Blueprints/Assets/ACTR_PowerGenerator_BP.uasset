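; Power generator actor that links to energy barriers and runs light-based checks with damage settings.
; Shortly after BeginPlay, it has each valid barrier in its light structure subscription component subscribe to the wall.
; Every tick it passes the damage multiplier and delay to LightComprobations.
; Construction matches the spotlight's outer cone to its inner angle and caches the health component; unconnected debug code draws the damage, safe-zone and exit spheres.
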(event EventBeginPlay
  ;[1 1 1] Begin Play
  (Utilities|FlowControl|Delay 0.2)
  (for _array_element (Variables|/Script/Voidout.ACMP_LightStructureSubscription|Getm_energyBarrier (Variables|Default|GetACMP_LightStructureSubscription))
    (Utilities|IsValid _array_element
      (:Is%20Valid
        (Class|ACTREnergyBarrier|SubscribetoWall _array_element)))))

(event EventTick
  (params (DeltaSeconds :type Float%20%28single-precision%29))
  ;[1 1 1] Tick
  (Class|ACTRLight|LightComprobations (Variables|Default|Getm_damageMultiplicator) DeltaSeconds (Variables|Default|Getm_delayUntilDamage)))

(fn ConstructionScript
  (bind _spotlight (Variables|Default|GetSpotLight))
  ;[1 1 1] Soluciona problemas de posicionamiento de las esferas de daño y para el movimiento de la IA.
  (Rendering|Lighting|SetOuterConeAngle _spotlight (Variables|/Script/Engine.SpotLightComponent|GetInnerConeAngle _spotlight))
  (Variables|Default|Setm_health (Actor|GetComponentbyClass "/Script/Voidout.ACMP_Health")))