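; One-shot save trigger that saves the game when the player overlaps its collision component.
; A helper function passes only if the trigger is unused, the actor is a CHRT_Player_BP and the overlapping component is a capsule, filtering out the player's other component types.
; On a pass it calls SaveGame on the player and sets Used to block further saves.
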(event OnComponentBeginOverlap(CollisionComponent)
  (params (OverlappedComponent :type Primitive%20Component%20Object%20Reference) (OtherActor :type Actor%20Object%20Reference) (OtherComp :type Primitive%20Component%20Object%20Reference) (OtherBodyIndex :type Integer) (bFromSweep :type Boolean) (SweepResult :type Hit%20Result%20Structure%20%28by%20ref%29))
  ;[1 1 1] Check if the Overlap is with a Player and it hasn't been used
  (bind (_return _aschrt_player) (CallFunction|IsActorPlayerandSaveNotUsed OtherActor OtherComp))
  (if _return
    ;[1 1 1] Saves and set Used value
    (Class|CHRTPlayer|SaveGame _aschrt_player)
    (Variables|Default|SetUsed true)))

(fn ConstructionScript)

(fn IsActorPlayerandSaveNotUsed
  (params (OtherActor :type Actor%20Object%20Reference) (OtherComp :type Actor%20Component%20Object%20Reference))
  (if (not (Variables|Default|GetUsed))
    (bind _aschrt_player_bp (Utilities|Casting|CastToCHRT_Player_BP OtherActor)
      (:then
        (Utilities|Casting|CastToCapsuleComponent OtherComp
          (:then
            (return true _aschrt_player_bp))
          (:CastFailed
            _)))
      (:CastFailed
        _))
    (return false 0)))