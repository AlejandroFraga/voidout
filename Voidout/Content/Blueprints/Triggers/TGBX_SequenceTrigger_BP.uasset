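; TGBX_SequenceTrigger_BP is a trigger Blueprint that starts and stops music for a sequence.
; Its StartMusicSequence and StopMusicSequence events each look up the SYST_SoundEventManager_BP actor and, if the Music variable is valid, call PlaySequenceMusic with a play or stop flag.
; The graph shows no overlap logic or caller for these events, and the construction script is empty.
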(event EventStartMusicSequence
  (bind _music (Variables|Default|GetMusic))
  ;[1 1 1] Controll Music Sequence
  (bind _returnvalue (Actor|GetActorOfClass "/Game/Blueprints/System/SYST_SoundEventManager_BP.SYST_SoundEventManager_BP_C"))
  (if (Utilities|IsValid _music)
    (Default|PlaySequenceMusic _returnvalue _music true)))

(event EventStopMusicSequence
  (bind _music (Variables|Default|GetMusic))
  ;[1 1 1] Controll Music Sequence
  (bind _returnvalue (Actor|GetActorOfClass "/Game/Blueprints/System/SYST_SoundEventManager_BP.SYST_SoundEventManager_BP_C"))
  (if (Utilities|IsValid _music)
    (Default|PlaySequenceMusic _returnvalue _music false)))

(fn ConstructionScript)