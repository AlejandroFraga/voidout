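; Trigger box that shows a tutorial page when the player's capsule overlaps it, selected by its tutorial ID.
; It updates the tutorial widget obtained from the player controller, and some IDs also permanently unlock Shadow Dash, directional Shadow Dash or Voidout.
; Most tutorials pause the game and destroy the trigger on entry.
; The first stays unpaused and is hidden, with the trigger destroyed, when the player leaves the volume.
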(event OnComponentBeginOverlap(CollisionComponent)
  (params (OverlappedComponent :type Primitive%20Component%20Object%20Reference) (OtherActor :type Actor%20Object%20Reference) (OtherComp :type Primitive%20Component%20Object%20Reference) (OtherBodyIndex :type Integer) (bFromSweep :type Boolean) (SweepResult :type Hit%20Result%20Structure%20%28by%20ref%29))
  (CallFunction|ComponentBeginOverlap OtherActor OtherComp))

(event OnComponentEndOverlap(CollisionComponent)
  (params (OverlappedComponent :type Primitive%20Component%20Object%20Reference) (OtherActor :type Actor%20Object%20Reference) (OtherComp :type Primitive%20Component%20Object%20Reference) (OtherBodyIndex :type Integer))
  (CallFunction|ComponentEndOverlap OtherActor OtherComp))

(fn ConstructionScript)

(fn GetGMINBase
  (bind _asgmin_base (Utilities|Casting|CastToGMIN_Base (Game|GetGameInstance))
    (:then
      (return _asgmin_base))
    (:CastFailed
      (return _asgmin_base))))

(fn GetCTRLPlayer
  (bind _returnvalue (Game|GetPlayerController 0))
  (Utilities|IsValid _returnvalue
    (:Is%20Valid
      (bind _asctrl_player_bp (Utilities|Casting|CastToCTRL_Player_BP _returnvalue)
        (:then
          (return _asctrl_player_bp))
        (:CastFailed
          _)))
    (:Is%20Not%20Valid
      _))
  (return 0))

(fn GetTutorial
  (bind _returnvalue (Game|GetPlayerController 0))
  (if (Utilities|IsValid _returnvalue)
    (bind _asctrl_player_bp (Utilities|Casting|CastToCTRL_Player_BP _returnvalue))
    (if (Utilities|IsValid _asctrl_player_bp)
      (if (Utilities|IsValid (Class|CTRLPlayer|GetTutorial _asctrl_player_bp))
        (bind _asuswg_tutorial (Utilities|Casting|CastToUSWG_Tutorial (Class|CTRLPlayer|GetTutorial _asctrl_player_bp)))
        (return _asuswg_tutorial)))))

(fn IsActorPlayer
  (params (OtherActor :type Actor%20Object%20Reference) (OtherComp :type Actor%20Component%20Object%20Reference))
  (Utilities|Casting|CastToCHRT_Player OtherActor
    (:then
      (Utilities|Casting|CastToCapsuleComponent OtherComp
        (:then
          (return true))
        (:CastFailed
          _)))
    (:CastFailed
      _))
  (return false))

(fn TutorialActions
  (params (tutorial :type USWG%20Tutorial%20Object%20Reference))
  (switch int (Variables|Default|GetidTutorial)
    (:1
      (Class|USWGMenuBase|UpdatePage tutorial "tutorial-01" false false))
    (:2
      (Class|USWGMenuBase|UpdatePage tutorial "tutorial-02" false false))
    (:3
      (Class|USWGMenuBase|UpdatePage tutorial "tutorial-03" false false))
    (:4
      (Class|USWGMenuBase|UpdatePage tutorial "tutorial-04" false false)
      ;[1 1 1] after this tutorial, the character can always use the ability
      (bind _asctrl_player (Utilities|Casting|CastToCTRL_Player (Game|GetPlayerController 0)))
      (Class|CTRLPlayer|UnlockShadowDash _asctrl_player))
    (:5
      (Class|USWGMenuBase|UpdatePage tutorial "tutorial-05" false false)
      ;[1 1 1] after this tutorial, the character can always use the ability with direction
      (bind _asctrl_player_2 (Utilities|Casting|CastToCTRL_Player (Game|GetPlayerController 0)))
      (Variables|/Script/Voidout.CTRL_Player|SetisDirectionalShadowDashUnlocked _asctrl_player_2 true))
    (:6
      (Class|USWGMenuBase|UpdatePage tutorial "tutorial-06" false false)
      ;[1 1 1] After this tutorial, the character can always use Voidout
      (bind _asctrl_player_3 (Utilities|Casting|CastToCTRL_Player (Game|GetPlayerController 0)))
      (Class|CTRLPlayer|UnlockVoidout _asctrl_player_3))
    (:7
      (Class|USWGMenuBase|UpdatePage tutorial "tutorial-07" false false))
    (:8
      (Class|USWGMenuBase|UpdatePage tutorial "tutorial-08" false false)))
  (return tutorial))

(fn ComponentBeginOverlap
  (params (otherActor :type Actor%20Object%20Reference) (otherComp :type Actor%20Component%20Object%20Reference))
  (bind _tutorial (CallFunction|GetTutorial))
  (bind _ctrlplayer (CallFunction|GetCTRLPlayer))
  (bind _idtutorial (Variables|Default|GetidTutorial))
  (bind _returnvalue (!= _idtutorial 1))
  (bind _isplayer (CallFunction|IsActorPlayer otherActor otherComp))
  (if _isplayer
    (Utilities|IsValid _tutorial
      (:Is%20Valid
        (CallFunction|TutorialActions _tutorial)
        (Utilities|IsValid _ctrlplayer
          (:Is%20Valid
            (Class|CTRLPlayer|ShowTutorial _ctrlplayer true _returnvalue _returnvalue)
            (if _returnvalue
              (Actor|DestroyActor)
              (else
                (Variables|Default|Setplayed true)))))))))

(fn ComponentEndOverlap
  (params (OtherActor :type Actor%20Object%20Reference) (OtherComp :type Actor%20Component%20Object%20Reference))
  (bind _ctrlplayer (CallFunction|GetCTRLPlayer))
  (if (Variables|Default|Getplayed)
    (bind _isplayer (CallFunction|IsActorPlayer OtherActor OtherComp))
    (if _isplayer
      (Utilities|IsValid _ctrlplayer
        (:Is%20Valid
          (Class|CTRLPlayer|ShowTutorial _ctrlplayer false false (!= (Variables|Default|GetidTutorial) 1))
          (Actor|DestroyActor))))))