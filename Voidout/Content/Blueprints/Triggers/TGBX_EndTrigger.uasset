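; TGBX_EndTrigger is a one-shot trigger box that starts music and calls End when the player enters it.
; On overlap it confirms the actor is a CHRT_Player and the overlapping component is a capsule, then sets Played to block repeats.
; It looks up SYST_SoundEventManager_BP in the level to play its Music event, then calls End, whose logic is not defined here.
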(event OnComponentBeginOverlap(CollisionComponent)
  (params (OverlappedComponent :type Primitive%20Component%20Object%20Reference) (OtherActor :type Actor%20Object%20Reference) (OtherComp :type Primitive%20Component%20Object%20Reference) (OtherBodyIndex :type Integer) (bFromSweep :type Boolean) (SweepResult :type Hit%20Result%20Structure%20%28by%20ref%29))
  (if (not (Variables|Default|Getplayed))
    (bind _isplayer (CallFunction|IsActorPlayer OtherActor OtherComp))
    (if _isplayer
      (Variables|Default|Setplayed true)
      (CallFunction|PlayMusicEvent)
      (Class|TGBXEndTrigger|End))))

(fn ConstructionScript)

(fn IsActorPlayer
  (params (OtherActor :type Actor%20Object%20Reference) (OtherComp :type Actor%20Component%20Object%20Reference))
  (bind _aschrt_player (Utilities|Casting|CastToCHRT_Player OtherActor)
    (:then
      (Utilities|Casting|CastToCapsuleComponent OtherComp
        (:then
          (return true _aschrt_player))
        (:CastFailed
          _)))
    (:CastFailed
      _))
  (return false 0))

(fn PlayMusicEvent
  (bind _returnvalue (Actor|GetActorOfClass "/Game/Blueprints/System/SYST_SoundEventManager_BP.SYST_SoundEventManager_BP_C"))
  (Default|PlayMusic _returnvalue true (Variables|Default|GetMusic)))