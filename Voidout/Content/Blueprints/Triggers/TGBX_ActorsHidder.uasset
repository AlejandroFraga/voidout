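; TGBX_ActorsHidder is a trigger box that reveals a set of hidden actors when the player enters it.
; On BeginPlay it hides every valid actor in ActorsToHide.
; An overlap on its collision component by a CHRT_Player capsule shows them all again, and nothing in the graph re-hides them afterwards.
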(event OnComponentBeginOverlap(CollisionComponent)
  (params (OverlappedComponent :type Primitive%20Component%20Object%20Reference) (OtherActor :type Actor%20Object%20Reference) (OtherComp :type Primitive%20Component%20Object%20Reference) (OtherBodyIndex :type Integer) (bFromSweep :type Boolean) (SweepResult :type Hit%20Result%20Structure%20%28by%20ref%29))
  (bind _isplayer (CallFunction|IsActorPlayer OtherActor OtherComp))
  (if _isplayer
    (CallFunction|HideAll false)))

(event EventBeginPlay
  (CallFunction|HideAll true))

(fn ConstructionScript)

(fn IsActorPlayer
  (params (OtherActor :type Actor%20Object%20Reference) (OtherComp :type Actor%20Component%20Object%20Reference))
  (Utilities|Casting|CastToCHRT_Player OtherActor
    (:then
      (Utilities|Casting|CastToCapsuleComponent OtherComp
        (:then
          (return true))
        (:CastFailed
          _)))
    (:CastFailed
      _))
  (return false))

(fn HideAll
  (params (Hide :type Boolean))
  (for _array_element (Variables|Default|GetactorsToHide)
    (Utilities|IsValid _array_element
      (:Is%20Valid
        (Rendering|SetActorHiddenInGame _array_element Hide))))
  (return))