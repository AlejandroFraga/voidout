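; AI controller for the Light Trooper enemy that starts its behavior tree on BeginPlay and tracks whether it senses the player.
; Perception updates for the player character write the sensed result to the canSeePlayer and Shoot blackboard keys.
; When sensing is lost, both keys are cleared unless the blackboard flags the player as marked by a flare, in which case they are left unchanged.
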(event OnTargetPerceptionUpdated(AIPerception)
  (params (Actor :type Actor%20Object%20Reference) (Stimulus :type AI%20Stimulus%20Structure))
  ;[1 1 1] If i can see the player, set the variable.
  (bind _output_get (Variables|Default|SetStimulusSuccessfullySensed (.bsuccessfullysensed Stimulus)))
  (Utilities|Casting|CastToCHRT_Player_BP Actor)
  (if _output_get
    (AI|Components|Blackboard|SetValueasBool (AI|GetBlackboard 0) (Utilities|Name|MakeLiteralName "canSeePlayer") (Variables|Default|GetStimulusSuccessfullySensed) :!label _label)
    (AI|Components|Blackboard|SetValueasBool (AI|GetBlackboard 0) (Utilities|Name|MakeLiteralName "Shoot") (Variables|Default|GetStimulusSuccessfullySensed))
    (elif (not (ScalableFloat|GetValueasBool (AI|GetBlackboard 0) (Utilities|Name|MakeLiteralName "PlayerMarkedByFlare")))
      (goto _label))))

(event EventBeginPlay
  (AI|RunBehaviorTree "/Game/Blueprints/BehaviourTree/BHTR_LightTrooper.BHTR_LightTrooper"))

(fn ConstructionScript)