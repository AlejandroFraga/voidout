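; AI controller for the Explorer character, which reacts to perceiving the player and flees.
; On BeginPlay it runs the BHTR_Explorer behavior tree.
; AI perception updates for the player trigger a nearby-enemy check and write the sensed state to the SeePlayer and PlayerNear blackboard keys.
; A successful sense also calls RunAwayFromPlayer.
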(event OnTargetPerceptionUpdated(AIPerception)
  (params (Actor :type Actor%20Object%20Reference) (Stimulus :type AI%20Stimulus%20Structure))
  (Utilities|Casting|CastToCHRT_Player_BP Actor)
  (Variables|Default|SetSensed (.bsuccessfullysensed Stimulus))
  (Class|AICTExplorer|CheckNearbyEnemy)
  (AI|Components|Blackboard|SetValueasBool (AI|GetBlackboard 0) (Utilities|Name|MakeLiteralName "SeePlayer") (Variables|Default|GetSensed))
  (AI|Components|Blackboard|SetValueasBool (AI|GetBlackboard 0) (Utilities|Name|MakeLiteralName "PlayerNear") (Variables|Default|GetSensed))
  (if (Variables|Default|GetSensed)
    (Class|AICTExplorer|RunAwayfromPlayer true)))

(event EventBeginPlay
  (AI|RunBehaviorTree "/Game/Blueprints/BehaviourTree/BHTR_Explorer.BHTR_Explorer"))

(fn ConstructionScript)