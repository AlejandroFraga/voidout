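; Player controller Blueprint that sets up the player's UI references and plays gamepad rumble for combat abilities.
; On BeginPlay it caches the Dark Slash and Marked By Flare indicators from the player pawn and registers a hidden pause menu widget.
; Force feedback functions for Voidout ready, Voidout explosion and Shadow Dash kill play only when the game instance reports controller use with vibration enabled.
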(event EventBeginPlay
  ;[1 1 1] Add the Visual Widgets
  (CallFunction|SetDarkSlash)
  (CallFunction|SetFlareIndicator)
  (CallFunction|AddPauseMenu)
  (|CallParentFunction))

(fn ConstructionScript)

(fn GetGMINBase
  (bind _asgmin_base (Utilities|Casting|CastToGMIN_Base (Game|GetGameInstance))
    (:then
      (return _asgmin_base))
    (:CastFailed
      (return _asgmin_base))))

(fn AddPauseMenu
  ;[1 1 1] Create and Set Pause Menu
  (bind _returnvalue (UserInterface|CreateWidget "/Game/Blueprints/UserWidget/Menu/USWG_PauseMenu.USWG_PauseMenu_C"))
  (bind _output_get (Variables|Default|SetpauseMenu _returnvalue))
  (Class|CTRLPlayer|AddMenu _output_get 998 false false false false)
  (return))

(fn SetDarkSlash
  ;[1 1 1] Create and Set Action Indicator
  (bind _aschrt_player_bp (Utilities|Casting|CastToCHRT_Player_BP (Pawn|GetControlledPawn)))
  (Variables|Default|SetdarkSlashIndicator (Variables|/Game/Blueprints/Character/CHRT_Player_BP.CHRT_Player_BP_C|GetDarkSlashIndicator _aschrt_player_bp))
  (return))

(fn SetFlareIndicator
  ;[1 1 1] Create and Set Action Indicator
  (bind _aschrt_player_bp (Utilities|Casting|CastToCHRT_Player_BP (Pawn|GetControlledPawn)))
  (Variables|Default|SetmarkedByFlareIndicator (Variables|/Game/Blueprints/Character/CHRT_Player_BP.CHRT_Player_BP_C|GetMarkedByFlareIndicator _aschrt_player_bp))
  (return))

(fn ForceFeedbackVoidoutReady
  (bind _gminbase (CallFunction|GetGMINBase))
  (if (and (Variables|/Script/Voidout.GMIN_Base|GetisUsingController _gminbase) (Variables|/Script/Voidout.GMIN_Base|GetisVibrationEnabled _gminbase))
    (Game|Feedback|ClientPlayForceFeedback (Game|GetPlayerController 0) "/Game/ForceFeedback/FFEF_VoidoutCooldown.FFEF_VoidoutCooldown" "Activated" false true true)
    (return)))

(fn ForceFeedbackVoidoutExplosion
  (bind _gminbase (CallFunction|GetGMINBase))
  (if (and (Variables|/Script/Voidout.GMIN_Base|GetisUsingController _gminbase) (Variables|/Script/Voidout.GMIN_Base|GetisVibrationEnabled _gminbase))
    (Game|Feedback|ClientPlayForceFeedback (Game|GetPlayerController 0) "/Game/ForceFeedback/FFEF_VoidoutExplosion.FFEF_VoidoutExplosion" "Activated" false true true)
    (return)))

(fn ForceFeedbackShadowDashKill
  (bind _gminbase (CallFunction|GetGMINBase))
  (if (and (Variables|/Script/Voidout.GMIN_Base|GetisUsingController _gminbase) (Variables|/Script/Voidout.GMIN_Base|GetisVibrationEnabled _gminbase))
    (Game|Feedback|ClientPlayForceFeedback (Game|GetPlayerController 0) "/Game/ForceFeedback/FFEF_ShadowDashKill.FFEF_ShadowDashKill" "Activated" false true true)
    (return)))