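; Shadow Explorer character Blueprint that supplies death sound and particle effects and caches its health component on construction.
; PlayDeathSound gets the sound event manager through the GMIN_Base game instance and plays the commander death sound at the actor's location.
; PlayDeathNPS activates the death and sparks particle systems, then triggers an event that deactivates both after a short delay.
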(event Custom|DeactiveNPSTimer
  (Utilities|FlowControl|Delay 1.0)
  (Components|Activation|Deactivate (Variables|Default|GetDeathNPS))
  (Components|Activation|Deactivate (Variables|Default|GetDeathSparksNPS)))

(fn ConstructionScript
  (Variables|Default|Setm_health (Actor|GetComponentbyClass "/Script/Voidout.ACMP_Health")))

(fn GetGMINBase
  (bind _asgmin_base (Utilities|Casting|CastToGMIN_Base (Game|GetGameInstance))
    (:then
      (return _asgmin_base))
    (:CastFailed
      (return _asgmin_base))))

(fn PlayDeathSound
  (bind _returnvalue (Class|GMINBase|GetSoundEventManager (CallFunction|GetGMINBase)))
  (Class|SYSTSoundEventManager|PlayCommanderDeath _returnvalue (Transformation|GetActorLocation))
  (return))

(fn PlayDeathNPS
  (Components|Activation|Activate (Variables|Default|GetDeathNPS) true)
  (Components|Activation|Activate (Variables|Default|GetDeathSparksNPS) true)
  (CallFunction|DeactiveNPSTimer)
  (return))