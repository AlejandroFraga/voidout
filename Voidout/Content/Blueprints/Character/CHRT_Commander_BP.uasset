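; Commander character Blueprint that can be assigned to an energy barrier and handles its own death effects.
; Shortly after BeginPlay it subscribes to the assigned barrier wall, then unsubscribes when destroyed.
; The construction script hands its EnergyShield to the health component.
; Death helpers play the commander sound through the game instance's sound event manager and fire two particle systems, deactivated after a short delay.
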(event Custom|DeactiveNPSTimer
  (Utilities|FlowControl|Delay 1.0)
  (Components|Activation|Deactivate (Variables|Default|GetDeathNPS))
  (Components|Activation|Deactivate (Variables|Default|GetDeathSparksNPS)))

(event EventBeginPlay
  (bind _m_energybarrierasigned (Variables|Default|Getm_energyBarrierAsigned))
  (Utilities|FlowControl|Delay 0.2)
  (Utilities|IsValid _m_energybarrierasigned
    (:Is%20Valid
      (Class|ACTREnergyBarrier|SubscribetoWall _m_energybarrierasigned))))

(event EventDestroyed
  (bind _m_energybarrierasigned (Variables|Default|Getm_energyBarrierAsigned))
  (Utilities|IsValid _m_energybarrierasigned
    (:Is%20Valid
      (Class|ACTREnergyBarrier|UnsubscribetoWall _m_energybarrierasigned))))

(fn ConstructionScript
  (bind _output_get (Variables|Default|Setm_health (Actor|GetComponentbyClass "/Script/Voidout.ACMP_Health")))
  (Variables|/Script/Voidout.ACMP_Health|Setm_energyShield _output_get (Variables|Default|GetEnergyShield)))

(fn PlayDeathSound
  (bind _returnvalue (Class|GMINBase|GetSoundEventManager (CallFunction|GetGMINBase)))
  (Class|SYSTSoundEventManager|PlayCommanderDeath _returnvalue (Transformation|GetActorLocation))
  (return))

(fn GetGMINBase
  (bind _asgmin_base (Utilities|Casting|CastToGMIN_Base (Game|GetGameInstance))
    (:then
      (return _asgmin_base))
    (:CastFailed
      (return _asgmin_base))))

(fn PlayDeathNPS
  (Components|Activation|Activate (Variables|Default|GetDeathNPS) true)
  (Components|Activation|Activate (Variables|Default|GetDeathSparksNPS) true)
  (CallFunction|DeactiveNPSTimer)
  (return))