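; Player character Blueprint that detects ability targets, drives damage feedback, and saves an initial checkpoint that it reloads on death.
; Range spheres for Dark Slash, Shadow Dash and Voidout forward overlaps to CTRL_Player, with line-of-sight checks on enemies entering the two attack spheres.
; A material parameter collection links health to the damage screen.
; Bullet hits spawn a direction widget, angled by dotting velocity against fixed 45-degree-yawed axes.
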(event OnComponentEndOverlap(ShadowDashReach)
  (params (OverlappedComponent :type Primitive%20Component%20Object%20Reference) (OtherActor :type Actor%20Object%20Reference) (OtherComp :type Primitive%20Component%20Object%20Reference) (OtherBodyIndex :type Integer))
  ;[1 1 1] When an enemy is in range to attack with first ability
  (CallFunction|OnSphereEndOverlapShadowDash OtherActor OtherComp))

(event OnComponentBeginOverlap(DarkSlashReach)
  (params (OverlappedComponent :type Primitive%20Component%20Object%20Reference) (OtherActor :type Actor%20Object%20Reference) (OtherComp :type Primitive%20Component%20Object%20Reference) (OtherBodyIndex :type Integer) (bFromSweep :type Boolean) (SweepResult :type Hit%20Result%20Structure%20%28by%20ref%29))
  ;[1 1 1] When an enemy is in range to attack with principal attack
  (CallFunction|OnSphereBeginOverlapDarkSlash OtherActor OtherComp))

(event OnComponentEndOverlap(DarkSlashReach)
  (params (OverlappedComponent :type Primitive%20Component%20Object%20Reference) (OtherActor :type Actor%20Object%20Reference) (OtherComp :type Primitive%20Component%20Object%20Reference) (OtherBodyIndex :type Integer))
  ;[1 1 1] When an enemy is in range to attack with principal attack
  (CallFunction|OnSphereEndOverlapDarkSlash OtherActor OtherComp))

(event OnComponentBeginOverlap(CapsuleComponent)
  (params (OverlappedComponent :type Primitive%20Component%20Object%20Reference) (OtherActor :type Actor%20Object%20Reference) (OtherComp :type Primitive%20Component%20Object%20Reference) (OtherBodyIndex :type Integer) (bFromSweep :type Boolean) (SweepResult :type Hit%20Result%20Structure%20%28by%20ref%29))
  ;[1 1 1] Damage direction HUD
  (CallFunction|DamageDirectionHUD OtherActor OtherComp SweepResult))

(event OnComponentBeginOverlap(VoidoutTowerSearcher)
  (params (OverlappedComponent :type Primitive%20Component%20Object%20Reference) (OtherActor :type Actor%20Object%20Reference) (OtherComp :type Primitive%20Component%20Object%20Reference) (OtherBodyIndex :type Integer) (bFromSweep :type Boolean) (SweepResult :type Hit%20Result%20Structure%20%28by%20ref%29))
  ;[1 1 1] When a tower is in range to use voidout ability
  (CallFunction|OnSphereBeginOverlapVoidout OtherActor OtherComp))

(event OnComponentEndOverlap(VoidoutTowerSearcher)
  (params (OverlappedComponent :type Primitive%20Component%20Object%20Reference) (OtherActor :type Actor%20Object%20Reference) (OtherComp :type Primitive%20Component%20Object%20Reference) (OtherBodyIndex :type Integer))
  ;[1 1 1] When a tower is in range to use voidout ability
  (CallFunction|OnSphereEndOverlapVoidout OtherActor OtherComp))

(event OnComponentBeginOverlap(ShadowDashReach)
  (params (OverlappedComponent :type Primitive%20Component%20Object%20Reference) (OtherActor :type Actor%20Object%20Reference) (OtherComp :type Primitive%20Component%20Object%20Reference) (OtherBodyIndex :type Integer) (bFromSweep :type Boolean) (SweepResult :type Hit%20Result%20Structure%20%28by%20ref%29))
  ;[1 1 1] When an enemy is in range to attack with first ability
  (CallFunction|OnSphereBeginOverlapShadowDash OtherActor OtherComp))

(event Custom|OnPlayerDeath
  ;[1 1 1] On Death Load Game
  (Class|CHRTPlayer|LoadGame))

(event EventBeginPlay
  ;[1 1 1] Initial Checkpoint
  (Utilities|FlowControl|Delay 0.2)
  (Class|CHRTPlayer|SaveGame))

(fn ConstructionScript
  (bind _output_get (Variables|Default|Setm_health (Actor|GetComponentbyClass "/Script/Voidout.ACMP_Health")))
  ;[1 1 1] Parameters to control damage screen USWG
  (Variables|/Script/Voidout.ACMP_Health|Setm_materialDamageCollection _output_get "/Game/Materials/HUD/DamageScreenParameterCollection.DamageScreenParameterCollection"))

(fn GetCTRLPlayer
  (bind _asctrl_player (Utilities|Casting|CastToCTRL_Player (Pawn|GetController)))
  (return _asctrl_player))

(fn ResetState
  (bind _controller (CallFunction|GetCTRLPlayer))
  (Class|ACMPFadeBlocking|CleanFadeObjects (Variables|Default|GetACMP_FadeBlocking))
  (if (Utilities|IsValid _controller)
    (Class|CTRLPlayer|ResetState _controller))
  (return))

(fn IsReachable
  (params (Actor :type Actor%20Object%20Reference))
  (Utilities|IsValid Actor
    (:Is%20Valid
      (bind _returnvalue (Collision|LineTraceByChannel (+ (Transformation|GetActorLocation) (Variables|Default|GetHeight)) (+ (Transformation|GetActorLocation Actor) (Variables|Default|GetHeight)) "TraceTypeQuery1" false (Utilities|Array|MakeArray Actor self) "None"))
      (return (not _returnvalue)))
    (:Is%20Not%20Valid
      (return false))))

(fn IsReachableEnemy
  (params (Actor :type Actor%20Object%20Reference))
  (bind _aschrt_enemy (Utilities|Casting|CastToCHRT_Enemy Actor)
    (:then
      (bind _output_get (LocalVariables|SetEnemyAux _aschrt_enemy))
      (Utilities|IsValid _output_get
        (:Is%20Valid
          (bind _returnvalue (CallFunction|IsReachable (LocalVariables|GetEnemyAux)))
          (return true _returnvalue (LocalVariables|GetEnemyAux)))
        (:Is%20Not%20Valid
          _)))
    (:CastFailed
      _))
  (return false false 0))

(fn OnSphereBeginOverlapDarkSlash
  (params (otherActor :type Actor%20Object%20Reference) (otherComp :type Actor%20Component%20Object%20Reference))
  (bind _controller (CallFunction|GetCTRLPlayer))
  (bind (_isenemy _reachable) (CallFunction|IsReachableEnemy otherActor))
  (if _isenemy
    (if _reachable
      (Utilities|IsValid _controller :!label _label
        (:Is%20Valid
          (Class|CTRLPlayer|OnSphereBeginOverlapDarkSlash _controller otherActor otherComp)
          (return))))
    (else
      (bind _asactr_destroyable_light (Utilities|Casting|CastToACTR_DestroyableLight otherActor))
      (Utilities|IsValid _asactr_destroyable_light
        (:Is%20Valid
          (goto _label))))))

(fn OnSphereEndOverlapDarkSlash
  (params (otherActor :type Actor%20Object%20Reference) (otherComp :type Actor%20Component%20Object%20Reference))
  (bind _controller (CallFunction|GetCTRLPlayer))
  (Utilities|IsValid _controller
    (:Is%20Valid
      (Class|CTRLPlayer|OnSphereEndOverlapDarkSlash _controller otherActor otherComp)
      (return))))

(fn OnSphereBeginOverlapShadowDash
  (params (otherActor :type Actor%20Object%20Reference) (otherComp :type Actor%20Component%20Object%20Reference))
  (bind _controller (CallFunction|GetCTRLPlayer))
  (bind (_isenemy _reachable) (CallFunction|IsReachableEnemy otherActor))
  (if (and _isenemy _reachable)
    (Utilities|IsValid _controller
      (:Is%20Valid
        (Class|CTRLPlayer|OnSphereBeginOverlapShadowDash _controller otherActor otherComp)
        (return)))))

(fn OnSphereEndOverlapShadowDash
  (params (otherActor :type Actor%20Object%20Reference) (otherComp :type Actor%20Component%20Object%20Reference))
  (bind _controller (CallFunction|GetCTRLPlayer))
  (Utilities|IsValid _controller
    (:Is%20Valid
      (Class|CTRLPlayer|OnSphereEndOverlapShadowDash _controller otherActor otherComp)
      (return))))

(fn OnSphereBeginOverlapVoidout
  (params (otherActor :type Actor%20Object%20Reference) (otherComponent :type Actor%20Component%20Object%20Reference))
  (bind _controller (CallFunction|GetCTRLPlayer))
  (if (Utilities|IsValid _controller)
    (Class|CTRLPlayer|OnTowerBeginOverlapVoidOut _controller otherActor otherComponent)))

(fn OnSphereEndOverlapVoidout
  (params (otherActor :type Actor%20Object%20Reference) (otherComponent :type Actor%20Component%20Object%20Reference))
  (bind _controller (CallFunction|GetCTRLPlayer))
  (if (Utilities|IsValid _controller)
    (Class|CTRLPlayer|OnTowerEndOverlapVoidOut _controller otherActor otherComponent)))

(fn ResetDamageScreen
  (Rendering|Material|SetScalarParameterValue "/Game/Materials/HUD/DamageScreenParameterCollection.DamageScreenParameterCollection" "Health" 1.0 :!class /Script/Engine.KismetMaterialLibrary)
  (return))

(fn GetifBullet
  (params (OtherActor :type Actor%20Object%20Reference) (OtherComp :type Actor%20Component%20Object%20Reference))
  (bind _asactr_bullet_bp (Utilities|Casting|CastToACTR_Bullet_BP OtherActor)
    (:then
      (Utilities|Casting|CastToCapsuleComponent OtherComp
        (:then
          (return true _asactr_bullet_bp))
        (:CastFailed
          _)))
    (:CastFailed
      _))
  (return false _asactr_bullet_bp))

(fn InitiateBulletVariables
  (params (ACTR%20Bullet%20BP :type ACTR%20Bullet%20BP%20Object%20Reference) (Sweep%20Result :type Hit%20Result%20Structure))
  (Variables|Default|SetbulletLocation (Transformation|GetActorLocation ACTR%20Bullet%20BP))
  (Variables|Default|Setvelocity (Transformation|GetVelocity ACTR%20Bullet%20BP))
  (Variables|Default|SethitPoint (.impactpoint Sweep%20Result))
  (return))

(fn CampleBulletMap
  (params (Condition2 :type Boolean) (Condition1 :type Boolean) (Value :type Float%20%28single-precision%29))
  (if Condition1
    (if Condition2
      ;[1 1 1] upper right
      (Variables|Default|Setangle (Math|Float|MapRangeClamped Value 0.0 1.0 0.25 0.5))
      (else
        ;[1 1 1] upper left
        (Variables|Default|Setangle (Math|Float|MapRangeClamped Value 0.0 1.0 0.75 0.5))))
    (elif Condition2
      ;[1 1 1] lower right
      (Variables|Default|Setangle (Math|Float|MapRangeClamped Value 0.0 -1.0 0.25 0.0))
      (else
        ;[1 1 1] lower left
        (Variables|Default|Setangle (Math|Float|MapRangeClamped Value 0.0 -1.0 0.75 1.0)))))
  (return))

(fn DamageDirectionHUD
  (params (OtherActor :type Actor%20Object%20Reference) (OtherComp :type Actor%20Component%20Object%20Reference) (Sweep%20Result :type Hit%20Result%20Structure))
  (bind _returnvalue (Math|Vector|GetRightVector "0,-45.000000, 0"))
  (bind _velocity (Variables|Default|Getvelocity))
  (bind _returnvalue_2 (Math|Vector|Normalize _velocity 0.001))
  (bind _returnvalue_3 (Math|Vector|DotProduct _returnvalue_2 _returnvalue))
  (bind (_isbullet _actr_bullet_bp) (CallFunction|GetifBullet OtherActor OtherComp))
  (if _isbullet
    (CallFunction|InitiateBulletVariables _actr_bullet_bp Sweep%20Result)
    (CallFunction|CampleBulletMap (<= (Math|Vector|DotProduct (Math|Vector|GetForwardVector "0,-45.000000, 0") _returnvalue_2) 0.0) (>= _returnvalue_3 0.0) _returnvalue_3)
    (bind _returnvalue_4 (UserInterface|CreateWidget "/Game/Blueprints/UserWidget/HUD/USWG_DamageDirection.USWG_DamageDirection_C" (Game|GetPlayerController 0) (Variables|Default|Getangle)))
    (UserInterface|Viewport|AddtoViewport _returnvalue_4 0)
    (return)))